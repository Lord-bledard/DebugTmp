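; Drake enemy Blueprint (BP_DarkeUsurper) that chases the player and plays a hand attack animation.
; PawnSensing sets a seen flag, never cleared here, and calls FollowPlayer, which runs AI Move To toward player 0 on each sighting.
; On arrival, a CanAttack gate leads to a delay before the montage, though every FollowPlayer call re-opens that gate.
; No damage logic is present.
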(event `self.PawnSensing.OnSeePawn`
  (params (Pawn :type "Pawn Object Reference"))
  (set `self.isSeeingP?` true)
  (`self.Follow Player`))

(event `Follow Player`
  (set `self.canAttack?` true)
  (if (`self.isSeeingP?`)
    (`|AIMoveTo` self (0.0 0.0 0.0) (`GameplayStatics.GetPlayerCharacter` 0) 70.0
      (:`OnSuccess`
        (if (`self.canAttack?`)
          (set `self.canAttack?` false)
          (`KismetSystemLibrary.Delay` 2.0)
          (`self.PlayAnimMontage` "/Game/FourEvilDragonsPBR/Animations/DragonTheUsurper/AttackHandAnim_Montage.AttackHandAnim_Montage")
          (set `self.canAttack?` true))))))

(fn `UserConstructionScript`)