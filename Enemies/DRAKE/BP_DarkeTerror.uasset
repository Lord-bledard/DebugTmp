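; Drake enemy pawn that chases the player and plays a flame-breath attack.
; PawnSensing's OnSeePawn sets a seeing flag, which this graph never clears, and calls FollowPlayer to AI-move toward player 0.
; On arrival, after a delay, it shows the Niagara effect with the flame montage, then hides it; no damage is applied here.
; FollowPlayer re-arms the CanAttack gate on every call.
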(event `self.ReceiveBeginPlay`
  (`SceneComponent.SetVisibility` (`self.Niagara`) false false))

(event `self.PawnSensing.OnSeePawn`
  (params (Pawn :type "Pawn Object Reference"))
  (set `self.isSeeingP?` true)
  (`self.Follow Player`))

(event `Follow Player`
  (set `self.canAttack?` true)
  (if (`self.isSeeingP?`)
    (`|AIMoveTo` self (0.0 0.0 0.0) (`GameplayStatics.GetPlayerCharacter` 0) 70.0
      (:`OnSuccess`
        (if (`self.canAttack?`)
          (set `self.canAttack?` false)
          (`KismetSystemLibrary.Delay` 2.0)
          (`SceneComponent.SetVisibility` (`self.Niagara`) true false)
          (`self.PlayAnimMontage` "/Game/FourEvilDragonsPBR/Animations/DragonTheTerrorBringer/AttackFlameAnim_Montage.AttackFlameAnim_Montage")
          (`KismetSystemLibrary.Delay` 2.0)
          (`SceneComponent.SetVisibility` (`self.Niagara`) false false)
          (set `self.canAttack?` true))))))

(fn `UserConstructionScript`)